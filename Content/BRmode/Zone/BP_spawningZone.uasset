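; Battle royale spawning zone actor that supplies random ground locations within a configurable box.
; On BeginPlay it registers itself with GM_BR as the SpawningZone, and its construction script sizes the Box from BoxExtent.
; GetRandomLocation line-traces WorldStatic objects downward from a random point in the box, returning the printed hit location or the actor's location on a miss.
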(event EventBeginPlay
  (bind _asgm_br (Utilities|Casting|CastToGM_BR (Game|GetGameMode)))
  (Variables|/Game/BRmode/GM_BR.GM_BR_C|SetspawningZone _asgm_br self))

(fn ConstructionScript
  (Components|Box|SetBoxExtent (Variables|Default|GetBox) (Variables|Default|GetboxExtent) true))

(fn GetRandomLocation
  (bind _returnvalue (Transformation|GetActorLocation))
  (bind _boxextent (Variables|Default|GetboxExtent))
  (bind _returnvalue_2 (Math|Random|RandomPointinBoundingBox _returnvalue _boxextent))
  (bind (_outhit _returnvalue_3) (Collision|LineTraceForObjects _returnvalue_2 (- _returnvalue_2 "0, 0,10000.000000") (Utilities|Array|MakeArray "ObjectTypeQuery1") false 0 "None"))
  (if _returnvalue_3
    (Development|PrintString (Utilities|String|ToString(Vector) (.Location (Collision|BreakHitResult _outhit))))
    (return (.Location (Collision|BreakHitResult _outhit)))
    (else
      (return _returnvalue))))