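; Battle royale game mode that gathers players and starts the match.
; PostLogin registers controllers up to a cap, removing extras; once the array index passes the fixed or minimum player threshold, it starts the countdown.
; The countdown scatters pawns to random SpawningZone points, then a named timer calls GameStart on the Zone.
; Zone spawning and the max-wait forced start are disconnected from BeginPlay, so never run.
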(event Custom|forceGameStart
  (bind _controllerarray (Variables|unconfigurable|GetControllerArray))
  (if (not (Class|KismetSystemLibrary|TimerExistsHandle (Variables|Unconfigurable|GetgameStartTimer)))
    (Utilities|FlowControl|Delay 1.0)
    (Development|PrintString (Utilities|String|Append "controller::" (Utilities|String|ToString(Integer) (Utilities|Array|Length _controllerarray))))
    (for _array_element _controllerarray
      (bind _aspc_fps (Utilities|Casting|CastToPC_FPS _array_element))
      (bind _location (Default|GetRandomLocation (Variables|Actors|GetspawningZone)))
      (Transformation|SetActorLocation (Variables|/Game/Blueprints/Characters/PC_FPS.PC_FPS_C|GetpawnRef _aspc_fps) _location false false))
    (bind _returnvalue (Utilities|Time|SetTimerbyFunctionName 0 "gameStart" (Variables|Config|GettimeBeforeGameStart)))
    (Variables|Unconfigurable|SetgameStartTimer _returnvalue)))

(event EventPostLogin
  (params (NewPlayer :type Player%20Controller%20Object%20Reference))
  (bind _controllerarray (Variables|unconfigurable|GetControllerArray))
  (bind _controllerarray_2 (Variables|unconfigurable|GetControllerArray))
  (bind _aspc_fps (Utilities|Casting|CastToPC_FPS NewPlayer))
  (if (< (Utilities|Array|Length _controllerarray) (Variables|Config|GetmaximumPlayer))
    (bind _returnvalue (Utilities|Array|Add _controllerarray _aspc_fps))
    (if (> _returnvalue (select (Variables|config|GetfixNbrPlayer) (Variables|Config|GetmaximumPlayer) (Variables|config|GetminimumPlayer)))
      (if (not (Class|KismetSystemLibrary|TimerExistsHandle (Variables|Unconfigurable|GetgameStartTimer)))
        (Utilities|FlowControl|Delay 1.0)
        (Development|PrintString (Utilities|String|Append "controller::" (Utilities|String|ToString(Integer) (Utilities|Array|Length _controllerarray_2))))
        (for _array_element _controllerarray_2
          (bind _aspc_fps_2 (Utilities|Casting|CastToPC_FPS _array_element))
          (bind _location (Default|GetRandomLocation (Variables|Actors|GetspawningZone)))
          (Transformation|SetActorLocation (Variables|/Game/Blueprints/Characters/PC_FPS.PC_FPS_C|GetpawnRef _aspc_fps_2) _location false false))
        (bind _returnvalue_2 (Utilities|Time|SetTimerbyFunctionName 0 "gameStart" (Variables|Config|GettimeBeforeGameStart)))
        (Variables|Unconfigurable|SetgameStartTimer _returnvalue_2)))
    (else
      (Class|GameplayStatics|RemovePlayer _aspc_fps true)
      (Development|PrintString "REMOVE PLAYER"))))

(event EventBeginPlay)

(event EventOnLogout
  (params (ExitingController :type Controller%20Object%20Reference))
  (bind _aspc_fps (Utilities|Casting|CastToPC_FPS ExitingController))
  (Utilities|Array|RemoveItem (Variables|unconfigurable|GetControllerArray) _aspc_fps)
  (Development|PrintString "REMOVE PLAYER"))

(fn ConstructionScript)

(fn GameStart
  (Default|GameStart (Variables|actors|Getzone) self))