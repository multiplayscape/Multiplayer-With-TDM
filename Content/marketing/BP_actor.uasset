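; Marketing mannequin actor that displays a character with a chosen team color, gun type and animation state.
; The construction script applies blue or red body materials and attaches the gun to a matching grip socket, using a static mesh for assault and handgun and a skeletal mesh for shotgun and sniper.
; On BeginPlay it copies the pose flags, walk speed and direction once into ABP_Marketing to drive the animation.
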(event EventBeginPlay
  (bind _asabp_marketing (Utilities|Casting|CastToABP_Marketing (Components|SkeletalMesh|GetAnimInstance (Variables|Default|GetSkeletalMesh))))
  (Variables|/Game/marketing/ABP_Marketing.ABP_Marketing_C|SetgunType _asabp_marketing (Variables|Default|GetgunType))
  (Variables|/Game/marketing/ABP_Marketing.ABP_Marketing_C|SetisCrouch _asabp_marketing (Variables|Default|GetisCrouch))
  (Variables|/Game/marketing/ABP_Marketing.ABP_Marketing_C|SetisReloading _asabp_marketing (Variables|Default|GetisReloading))
  (Variables|/Game/marketing/ABP_Marketing.ABP_Marketing_C|SetSpeed _asabp_marketing (Variables|Default|GetspeedWalk))
  (Variables|/Game/marketing/ABP_Marketing.ABP_Marketing_C|Setdirection _asabp_marketing (Variables|Default|GetdirectionWalk))
  (Variables|/Game/marketing/ABP_Marketing.ABP_Marketing_C|SetisMelee _asabp_marketing (Variables|Default|GetisMelee))
  (Variables|/Game/marketing/ABP_Marketing.ABP_Marketing_C|SetisThrowing _asabp_marketing (Variables|Default|GetisThrowing)))

(fn ConstructionScript
  (bind _returnvalue (Math|Transform|MakeTransform "0, 0, 0"))
  (bind _isbluecolor (Variables|Default|GetisBlueColor))
  (bind _skeletalmesh (Variables|Default|GetSkeletalMesh))
  (bind _skeletalmesh_2 (Variables|Default|GetSkeletalMesh))
  (bind _guntype (Variables|Default|GetgunType))
  (bind _returnvalue_2 (Utilities|Select :Index _guntype :NewEnumerator0 "GripPoint" :NewEnumerator1 "GripPoint_shotgun" :NewEnumerator2 "GripPoint_sniper" :NewEnumerator3 "GripPoint_handgun"))
  (for _index (range 0 (- (Rendering|Material|GetNumMaterials _skeletalmesh) 1))
    (Rendering|Material|SetMaterial _skeletalmesh _index (Utilities|Select :Index _index :Option%200 (select _isbluecolor "/Game/Meshes/characters/Materials/ThirdPerson/M_UE4Man_Body_Blue.M_UE4Man_Body_Blue" "/Game/Meshes/characters/Materials/ThirdPerson/M_UE4Man_Body_Red.M_UE4Man_Body_Red") :Option%201 (select _isbluecolor "/Game/Meshes/characters/Materials/ThirdPerson/M_UE4Man_ChestLogo_Blue.M_UE4Man_ChestLogo_Blue" "/Game/Meshes/characters/Materials/ThirdPerson/M_UE4Man_ChestLogo_Red.M_UE4Man_ChestLogo_Red"))))
  (switch Utilities|FlowControl|Switch|SwitchongunTypeEnum _guntype
    (:NewEnumerator0
      (bind _returnvalue_3 (AddComponent|AddStaticMeshComponent true _returnvalue :!label _label))
      (Components|StaticMesh|SetStaticMesh _returnvalue_3 (Utilities|Select :Index _guntype :NewEnumerator0 "/Game/Meshes/Weapons/assault/assault.assault" :NewEnumerator1 0 :NewEnumerator2 0 :NewEnumerator3 "/Game/Meshes/Weapons/handgun/handgun.handgun"))
      (Transformation|AttachComponentToComponent _returnvalue_3 _skeletalmesh_2 _returnvalue_2 "KeepRelative" "KeepRelative" "KeepRelative" true))
    (:NewEnumerator1
      (bind _returnvalue_4 (AddComponent|AddSkeletalMeshComponent true _returnvalue :!label _label_2))
      (Class|SkinnedMeshComponent|SetSkeletalMesh _returnvalue_4 (Utilities|Select :Index _guntype :NewEnumerator0 0 :NewEnumerator1 "/Game/Meshes/Weapons/shotgun/Shotgun_Reload_GUN_A.Shotgun_Reload_GUN_A" :NewEnumerator2 "/Game/Meshes/Weapons/sniper/Sniper_Reload_GUN.Sniper_Reload_GUN" :NewEnumerator3 0) true)
      (Transformation|AttachComponentToComponent _returnvalue_4 _skeletalmesh_2 _returnvalue_2 "KeepRelative" "KeepRelative" "KeepRelative" true))
    (:NewEnumerator2
      (goto _label_2))
    (:NewEnumerator3
      (goto _label))))