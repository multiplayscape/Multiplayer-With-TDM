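; Player controller for the multiplayer FPS that handles team spawning, chat and match UI for each player.
; BeginPlay queries GM_FPS for the game mode to build the spawn screen and scoreboard, and TeamSelected spawns the pawn through it.
; Chat loops over the game mode's controllers, filtering by team for team messages.
; Other events relay score, timer and win/lose results to HUD widgets, and trigger zone effects and platforms.
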(event Custom|TeamSelected
  (params (Team :type Teams%20Enum :default "NewEnumerator0") (gunType :type gunTypeEnum%20Enum :default "NewEnumerator0"))
  ;[1 0.8542 0] Set [Team] & Spawn Player
  (Variables|Default|SetisReady true)
  (bind _output_get (Variables|Default|SetTeam Team))
  (bind _asgm_fps (Utilities|Casting|CastToGM_FPS (Game|GetGameMode)))
  (bind _asbp_fps (Utilities|Casting|CastToBP_FPS (Pawn|GetControlledPawn)))
  (Variables|/Game/Blueprints/Characters/BP_FPS.BP_FPS_C|SetTeam _asbp_fps (Variables|Default|GetTeam))
  (bind _bp_fpsref (Default|SpawnTeamSelect _asgm_fps _output_get gunType self _asbp_fps))
  (Collision|SetCollisionEnabled (Variables|/Script/Engine.Character|GetMesh _bp_fpsref) "QueryAndPhysics")
  (Variables|Default|SetpawnRef _bp_fpsref))

(event Custom|SetWidgetPawnRef
  (params (PlayerRef :type BP%20FPS%20Object%20Reference) (Index :type Teams%20Enum :default "NewEnumerator0"))
  ;[0 0.4075 1] Set {HUD_FPS} Ref
  (bind _ashud_fps (Utilities|Casting|CastToHUD_FPS (HUD|GetHUD)))
  (Variables|/Game/UMG/Widgets/W_HUD.W_HUD_C|SetPlayerREF (Variables|/Game/Blueprints/HUD_FPS.HUD_FPS_C|GetHUDWidgetREF _ashud_fps) PlayerRef)
  (Widget|SetVisibility (Variables|/Game/UMG/Widgets/W_HUD.W_HUD_C|GetteamSelect (Variables|/Game/Blueprints/HUD_FPS.HUD_FPS_C|GetHUDWidgetREF _ashud_fps)) (select (Utilities|Enum|Equal(Enum) Index "NewEnumerator0") "Collapsed" "Visible"))
  (Class|Image|SetBrushfromMaterial (Variables|/Game/UMG/Widgets/W_HUD.W_HUD_C|GetteamSelect (Variables|/Game/Blueprints/HUD_FPS.HUD_FPS_C|GetHUDWidgetREF _ashud_fps)) (Utilities|Select :Index Index :NewEnumerator0 0 :NewEnumerator1 "/Game/UMG/Textures/UI/team/teamLogo_Mat_Inst.teamLogo_Mat_Inst" :NewEnumerator2 "/Game/UMG/Textures/UI/team/teamLogo_Mat_Inst1.teamLogo_Mat_Inst1")))

(event Custom|BR_reverseEffect
  (CallFunction|BRClientReverseEffect (Variables|Default|Getzone)))

(event Custom|createScoreBoard
  (params (isTeam :type Boolean) (gameMode :type Gamemodes%20Enum :default "NewEnumerator0"))
  ;[0 0 1] Begin Play
  (bind _ashud_fps (Utilities|Casting|CastToHUD_FPS (HUD|GetHUD)))
  (Default|CreateScoreBoard _ashud_fps isTeam gameMode))

(event Custom|askScoreboard
  ;[0 0 1] Begin Play
  (bind _asgm_fps (Utilities|Casting|CastToGM_FPS (Game|GetGameMode)))
  (CallFunction|CreateScoreBoard (Utilities|Select :Index (Variables|/Game/Blueprints/GameMode/GM_FPS.GM_FPS_C|GetMode _asgm_fps) :NewEnumerator0 false :NewEnumerator1 true :NewEnumerator2 true :NewEnumerator3 true :NewEnumerator4 true) (Variables|/Game/Blueprints/GameMode/GM_FPS.GM_FPS_C|GetMode _asgm_fps)))

(event Custom|displayEndGAme
  (params (WinnerName :type String) (isDraw :type Boolean) (isWin :type Boolean) (Target :type BP%20FPS%20Object%20Reference))
  (bind _spawnscreen (Variables|Default|GetSpawnScreen))
  (bind _hudref (Variables|/Game/Blueprints/Characters/BP_FPS.BP_FPS_C|GetHUDREF Target))
  (bind _respawnscreenref (Variables|/Game/Blueprints/HUD_FPS.HUD_FPS_C|GetRespawnScreenREF _hudref))
  ;[0.5791 0.0547 1] After Game finishes, declare Winner and losers
  (Utilities|IsValid _respawnscreenref
    (:Is%20Valid
      (Widget|SetVisibility _respawnscreenref "Collapsed"))
    (:Is%20Not%20Valid
      _))
  (Utilities|IsValid _spawnscreen
    (:Is%20Valid
      (Widget|SetVisibility _spawnscreen "Collapsed"))
    (:Is%20Not%20Valid
      _))
  (bind _returnvalue (UserInterface|CreateWidget "/Game/UMG/Widgets/W_gameEnd.W_gameEnd_C" 0 isDraw isWin))
  (UserInterface|Viewport|AddtoViewport _returnvalue 0))

(event Custom|setPawnServer
  (params (pawnRef :type BP%20FPS%20Object%20Reference))
  ;[1 1 1] Comment
  (Variables|Default|SetpawnRef pawnRef))

(event Custom|askGameMode
  ;[0 0 1] Begin Play
  (bind _asgm_fps (Utilities|Casting|CastToGM_FPS (Game|GetGameMode)))
  (CallFunction|CreateSpawnScreen (Variables|/Game/Blueprints/GameMode/GM_FPS.GM_FPS_C|GetMode _asgm_fps)))

(event Custom|gameReady
  (CallFunction|DisplayTimer true))

(event Custom|displayTimer
  (params (isGameStart :type Boolean))
  (bind _ashud_fps (Utilities|Casting|CastToHUD_FPS (HUD|GetHUD)))
  (Utilities|IsValid _ashud_fps
    (:Is%20Valid
      (Default|DisplayTimer (Variables|/Game/Blueprints/HUD_FPS.HUD_FPS_C|GetTimer%20REF _ashud_fps) isGameStart))))

(event Custom|gameOver
  (CallFunction|DisplayTimer false))

(event Custom|updateQuickScoreboard
  (params (isOwn :type Boolean) (team :type Teams%20Enum :default "NewEnumerator0") (Target :type BP%20FPS%20Object%20Reference) (score :type Integer))
  (bind _returnvalue (Utilities|Enum|Equal(Enum) team "NewEnumerator0"))
  (bind _team (Variables|Default|GetTeam))
  (bind _hudref (Variables|/Game/Blueprints/Characters/BP_FPS.BP_FPS_C|GetHUDREF Target))
  (bind _returnvalue_2 (Utilities|Enum|Equal(Enum) team _team))
  (bind _hudwidgetref (Variables|/Game/Blueprints/HUD_FPS.HUD_FPS_C|GetHUDWidgetREF _hudref))
  (bind _scoreother (Variables|/Game/UMG/Widgets/W_HUD.W_HUD_C|GetscoreOther _hudwidgetref))
  (bind _scoreown (Variables|/Game/UMG/Widgets/W_HUD.W_HUD_C|GetscoreOwn _hudwidgetref))
  (bind _returnvalue_3 (select isOwn _scoreown _scoreother))
  (bind _returnvalue_4 (select _returnvalue_2 _scoreown _scoreother))
  (bind _returnvalue_5 (select _returnvalue _returnvalue_3 _returnvalue_4))
  (bind _returnvalue_6 (Class|TextBlock|GetText _returnvalue_5))
  (bind _returnvalue_7 (Utilities|String|ToString(Text) _returnvalue_6))
  (bind _returnvalue_8 (Math|Conversions|ToInteger(Byte) _returnvalue_7))
  (bind _returnvalue_9 (+ _returnvalue_8 1))
  (bind _returnvalue_10 (Utilities|Text|ToText(Integer) _returnvalue_9))
  ;[1 1 1] update small scoreboard
  (if _returnvalue
    (if isOwn
      (Rendering|Components|TextRender|SetText _scoreown _returnvalue_10)
      (elif (> score (Math|Conversions|ToInteger(Byte) (Utilities|String|ToString(Text) (Class|TextBlock|GetText _scoreother))))
        (Rendering|Components|TextRender|SetText _scoreother (Utilities|Text|ToText(Integer) score))))
    (else
      (Rendering|Components|TextRender|SetText _returnvalue_5 _returnvalue_10))))

(event Custom|GetChatMessage
  (params (SenderText :type Text))
  ;[1 0 0.8789] Send message to every active player in the lobby // every teammates in the lobby
  (bind _asgm_fps (Utilities|Casting|CastToGM_FPS (Game|GetGameMode)))
  (if (Variables|Default|GetTeamChatMessage)
    (for _array_element (Variables|/Game/Blueprints/GameMode/GM_FPS.GM_FPS_C|GetControllerArray _asgm_fps)
      (bind _aspc_fps (Utilities|Casting|CastToPC_FPS _array_element))
      (if (Utilities|Enum|Equal(Enum) (Variables|PC_FPS_C|GetTeam _aspc_fps) (Variables|Default|GetTeam)) ; Distinguish teams
        (CallFunction|UpdateChat _aspc_fps (Variables|Default|GetPlayerName) (Variables|Default|GetTeamChatMessage) SenderText) ; Team Chat
      ))
    (else
      (for _array_element_2 (Variables|/Game/Blueprints/GameMode/GM_FPS.GM_FPS_C|GetControllerArray _asgm_fps)
        (bind _aspc_fps_2 (Utilities|Casting|CastToPC_FPS _array_element_2))
        (CallFunction|UpdateChat _aspc_fps_2 (Variables|Default|GetPlayerName) (Variables|Default|GetTeamChatMessage) SenderText) ; Global Chat
      ))))

(event Custom|updateQuickScoreboardCall
  (params (isOwn :type Boolean) (team :type Teams%20Enum :default "NewEnumerator0") (score :type Integer))
  ;[1 1 1] update small scoreboard
  (CallFunction|UpdateQuickScoreboard isOwn team (Variables|Default|GetpawnRef) score))

(event Custom|WinningServer
  (params (WinnerName :type String) (isDraw :type Boolean))
  ;[0.5791 0.0547 1] After Game finishes, declare Winner and losers
  (CallFunction|DisplayEndGAme WinnerName isDraw true (Variables|Default|GetpawnRef)))

(event Custom|LosingServer
  (params (Loser%20name :type String))
  ;[0.5791 0.0547 1] After Game finishes, declare Winner and losers
  (CallFunction|DisplayEndGAme Loser%20name false false (Variables|Default|GetpawnRef)))

(event Custom|BR_ClientPlayEffect
  (params (ZoneRef :type Zone%20Object%20Reference))
  (Default|PlayEffects ZoneRef))

(event Custom|updateScoreboard
  (params (Target :type BP%20FPS%20Object%20Reference) (Index :type Teams%20Enum :default "NewEnumerator0"))
  (bind _hudref (Variables|/Game/Blueprints/Characters/BP_FPS.BP_FPS_C|GetHUDREF Target))
  (bind _scoreboardref (Variables|/Game/Blueprints/HUD_FPS.HUD_FPS_C|GetScoreboardREF _hudref))
  (bind _scoreleft (Variables|/Game/UMG/Widgets/W_ScoreBoard.W_ScoreBoard_C|GetScoreLeft _scoreboardref))
  (bind _scoreright (Variables|/Game/UMG/Widgets/W_ScoreBoard.W_ScoreBoard_C|GetscoreRight _scoreboardref))
  (bind _returnvalue (Utilities|Select :Index Index :NewEnumerator0 0 :NewEnumerator1 _scoreleft :NewEnumerator2 _scoreright))
  (Rendering|Components|TextRender|SetText _returnvalue (Utilities|Text|ToText(Integer) (+ (Math|Conversions|ToInteger(Byte) (Utilities|String|ToString(Text) (Class|TextBlock|GetText _returnvalue))) 1))))

(event Custom|updateScoreboardCall
  (params (team :type Teams%20Enum :default "NewEnumerator0"))
  ;[1 1 1] update small scoreboard
  (CallFunction|UpdateScoreboard (Variables|Default|GetpawnRef) team))

(event Custom|Set%20Player%20ID
  ;[0 0 1] Begin Play
  (if (not (Networking|IsServer))
    (Utilities|IsValid (Variables|Default|Getgameinstanceref)
      (:Is%20Not%20Valid
        (bind _asmultiplayer_game_instance (Utilities|Casting|CastToMultiplayerGameInstance (Game|GetGameInstance)))
        (bind _output_get (Variables|Default|Setgameinstanceref _asmultiplayer_game_instance))
        (Variables|Default|SetPlayerName (Variables|/Game/FirstPersonBP/Blueprints/MultiplayerGameInstance.MultiplayerGameInstance_C|Getplayer%20id _output_get))))))

(event Custom|UpdateChat
  (params (playerName :type String) (TeamChat%20? :type Boolean) (text :type Text))
  ;[1 0 0.9075] Set {W_ChatBox} if a message has been sent / recieved
  (bind _ashud_fps (Utilities|Casting|CastToHUD_FPS (HUD|GetHUD)))
  (Default|UpdateChat (Variables|/Game/UMG/Widgets/W_HUD.W_HUD_C|GetW_ChatBox (Variables|/Game/Blueprints/HUD_FPS.HUD_FPS_C|GetHUDWidgetREF _ashud_fps)) (Variables|Default|GetTeam) TeamChat%20? playerName text) ; This will need a PlayerName
  (Class|Border|SetBrushColor (Variables|/Game/UMG/Widgets/W_ChatBox.W_ChatBox_C|GetChatContainer (Variables|/Game/UMG/Widgets/W_HUD.W_HUD_C|GetW_ChatBox (Variables|/Game/Blueprints/HUD_FPS.HUD_FPS_C|GetHUDWidgetREF _ashud_fps))) (select (Variables|/Game/UMG/Widgets/W_ChatBox.W_ChatBox_C|GetisOpen (Variables|/Game/UMG/Widgets/W_HUD.W_HUD_C|GetW_ChatBox (Variables|/Game/Blueprints/HUD_FPS.HUD_FPS_C|GetHUDWidgetREF _ashud_fps))) "(R=0.000000,G=0.000000,B=0.000000,A=0.250000)" "(R=0.000000,G=0.000000,B=0.000000,A=0.000000)"))
  (Widget|SetVisibility (Variables|/Game/UMG/Widgets/W_HUD.W_HUD_C|GetW_ChatBox (Variables|/Game/Blueprints/HUD_FPS.HUD_FPS_C|GetHUDWidgetREF _ashud_fps)) "Visible")
  (if (not (Variables|/Game/UMG/Widgets/W_ChatBox.W_ChatBox_C|GetisOpen (Variables|/Game/UMG/Widgets/W_HUD.W_HUD_C|GetW_ChatBox (Variables|/Game/Blueprints/HUD_FPS.HUD_FPS_C|GetHUDWidgetREF _ashud_fps))))
    (Default|VisibilityTimer (Variables|/Game/UMG/Widgets/W_HUD.W_HUD_C|GetW_ChatBox (Variables|/Game/Blueprints/HUD_FPS.HUD_FPS_C|GetHUDWidgetREF _ashud_fps)))))

(event Custom|PlatformCallOnPC
  (params (obj :type Array%20of%20Platform%20Object%20References))
  ;[0.0999 0.08961 1] Platform - On all Clients
  (for _array_element obj
    (Default|Start _array_element)))

(event Custom|SetTeamChatMessage
  (params (TeamChatMessage :type Boolean))
  ;[1 0 0.8789] Send message to every active player in the lobby // every teammates in the lobby
  ;;[1 0 0 1 14] Set Boolean value on server
  (Variables|Default|SetTeamChatMessage TeamChatMessage))

(event Custom|BR_PlayEffectsOnStart
  (CallFunction|BRClientPlayEffect (Variables|Default|Getzone)))

(event Custom|BR_clientReverseEffect
  (params (ZoneRef :type Zone%20Object%20Reference))
  (Default|ReverseEffect ZoneRef))

(event Custom|BR_PlayEffect
  (CallFunction|BRClientPlayEffect (Variables|Default|Getzone)))

(event Custom|createSpawnScreen
  (params (gameMode :type Gamemodes%20Enum :default "NewEnumerator0"))
  ;[0 0 1] Begin Play
  (bind _returnvalue (UserInterface|CreateWidget "/Game/UMG/Widgets/W_SpawnScreen.W_SpawnScreen_C" 0 gameMode))
  (bind _output_get (Variables|Default|SetSpawnScreen _returnvalue))
  (UserInterface|Viewport|AddtoViewport _output_get 0)
  (Variables|Default|SetbShowMouseCursor true))

(event EventBeginPlay
  ;[0 0 1] Begin Play
  (if (Pawn|IsLocalController)
    (CallFunction|AskGameMode)
    (CallFunction|AskScoreboard)
    (CallFunction|SetPlayerID)))

(fn ConstructionScript)