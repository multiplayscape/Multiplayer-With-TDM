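; Moving platform actor that slides its static mesh back and forth between the first two points of a spline.
; A timeline lerps the mesh position, with Start setting play rate from the Time variable, and a timer on finish flip-flops direction after a pause.
; On BeginPlay it passes all Platform actors to the GM_FPS game mode.
; The construction script places the mesh at the IndexTesting spline point for previewing.
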(event Custom|Back
  (bind _spline (Variables|Default|GetSpline))
  (bind _newtrack_0 (Timeline|Timeline_0 Reverse)
    (:Update
      (Transformation|SetWorldLocation (Variables|Default|GetStaticMesh) (Math|Vector|Lerp(Vector) (Spline|GetLocationatSplinePoint _spline 0 "World") (Spline|GetLocationatSplinePoint _spline 1 "World") _newtrack_0) false false))
    (:Finished
      (Utilities|Time|SetTimerbyEvent (delegate Custom|Timer) 3.0))))

(event Custom|Forward
  (bind _spline (Variables|Default|GetSpline))
  (bind _newtrack_0 (Timeline|Timeline_0 Play)
    (:Update
      (Transformation|SetWorldLocation (Variables|Default|GetStaticMesh) (Math|Vector|Lerp(Vector) (Spline|GetLocationatSplinePoint _spline 0 "World") (Spline|GetLocationatSplinePoint _spline 1 "World") _newtrack_0) false false))
    (:Finished
      (Utilities|Time|SetTimerbyEvent (delegate Custom|Timer) 3.0))))

(event Custom|Timer
  (Utilities|FlowControl|FlipFlop
    (:A
      (CallFunction|Back))
    (:B
      (CallFunction|Forward))))

(event Custom|Start
  (bind _spline (Variables|Default|GetSpline))
  (Components|Timeline|SetPlayRate (Variables|Default|GetTimeline_0) (/ 1.0 (Variables|Default|Gettime)))
  (bind _newtrack_0 (Timeline|Timeline_0 Play)
    (:Update
      (Transformation|SetWorldLocation (Variables|Default|GetStaticMesh) (Math|Vector|Lerp(Vector) (Spline|GetLocationatSplinePoint _spline 0 "World") (Spline|GetLocationatSplinePoint _spline 1 "World") _newtrack_0) false false))
    (:Finished
      (Utilities|Time|SetTimerbyEvent (delegate Custom|Timer) 3.0))))

(event EventBeginPlay
  (bind _asgm_fps (Utilities|Casting|CastToGM_FPS (Game|GetGameMode)))
  (bind _outactors (Actor|GetAllActorsOfClass "Platform_C"))
  (Default|PlatformCall _asgm_fps _outactors))

(fn ConstructionScript
  (Transformation|SetWorldLocation (Variables|Default|GetStaticMesh) (Spline|GetLocationatSplinePoint (Variables|Default|GetSpline) (Variables|Default|GetIndexTesting) "World") false false))