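; AmmoBox is a world pickup that refills ammo for the BP_FPS player's equipped weapon on overlap, unless they are reloading.
; Calculate picks the primary or secondary weapon and adds a third of its capacity to current ammo, clamped to capacity.
; The overlap event passes the result to UpdateAmmo and the weapon's struct.
; The box hides and becomes unavailable, then reactivates after a fixed delay.
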(event OnComponentBeginOverlap(Box)
  (params (OverlappedComponent :type Primitive%20Component%20Object%20Reference) (OtherActor :type Actor%20Object%20Reference) (OtherComp :type Primitive%20Component%20Object%20Reference) (OtherBodyIndex :type Integer) (bFromSweep :type Boolean) (SweepResult :type Hit%20Result%20Structure%20%28by%20ref%29))
  (if (Variables|Default|GetBoxAvailable)
    (bind _asbp_fps (Utilities|Casting|CastToBP_FPS OtherActor))
    (Variables|Default|SetBPFPSRef _asbp_fps)
    (if (not (Variables|/Game/Blueprints/Characters/BP_FPS.BP_FPS_C|GetIsReloading _asbp_fps))
      ;[1 1 1] Deactivate AmmoBox
      (Rendering|SetVisibility (Variables|Default|GetBox) false false)
      (Variables|Default|SetBoxAvailable false)
      (Default|UpdateAmmo (Variables|Default|GetBPFPSRef) (.Ammo (Utilities|Calculate (Variables|Default|GetBPFPSRef))))
      (bind _structout (Utilities|Struct|SetmembersinWeaponStruct (.WeaponStructure (Utilities|Calculate (Variables|Default|GetBPFPSRef))) (.Ammo (Utilities|Calculate (Variables|Default|GetBPFPSRef)))))
      (Variables|/Game/Blueprints/Weapons/_WeaponMaster._WeaponMaster_C|SetWeaponStructure (.ReturnValue (Utilities|Calculate (Variables|Default|GetBPFPSRef))) _structout)
      ;[1 1 1 1 16] Delay for AmmoBox to Reactivate
      (Utilities|FlowControl|Delay 1e+01)
      ;[1 1 1] Reactivate AmmoBox
      (Rendering|SetVisibility (Variables|Default|GetBox) true false)
      (Variables|Default|SetBoxAvailable true))))

(fn ConstructionScript)