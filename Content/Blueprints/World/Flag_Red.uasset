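; Red team flag actor for a capture-the-flag mode, which records its starting location at BeginPlay.
; When a Blue BP_FPS capsule overlaps the flag mesh, the flag snaps to that player's "head" socket and sets HasEnemyFlag.
; A Red player carrying the enemy flag triggers ScorePoint, which only teleports this flag to its start, without updating score or carrier state.
; FlagDrop is an empty stub.
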(event OnComponentBeginOverlap(FlagMesh)
  (params (OverlappedComponent :type Primitive%20Component%20Object%20Reference) (OtherActor :type Actor%20Object%20Reference) (OtherComp :type Primitive%20Component%20Object%20Reference) (OtherBodyIndex :type Integer) (bFromSweep :type Boolean) (SweepResult :type Hit%20Result%20Structure%20%28by%20ref%29))
  (bind _asbp_fps (Utilities|Casting|CastToBP_FPS OtherActor))
  (if (== (Variables|/Script/Engine.Character|GetCapsuleComponent _asbp_fps) OtherComp)
    (switch Utilities|FlowControl|Switch|SwitchonTeams (Variables|/Game/Blueprints/Characters/BP_FPS.BP_FPS_C|GetTeam _asbp_fps)
      (:NewEnumerator1
        (Transformation|AttachActorToActor _asbp_fps "head" "SnapToTarget" "SnapToTarget" "SnapToTarget" true)
        (Variables|/Game/Blueprints/Characters/BP_FPS.BP_FPS_C|SetHasEnemyFlag _asbp_fps true))
      (:NewEnumerator2
        (if (Variables|/Game/Blueprints/Characters/BP_FPS.BP_FPS_C|GetHasEnemyFlag _asbp_fps)
          (CallFunction|ScorePoint))))))

(event Custom|ScorePoint
  (Transformation|SetActorLocation (Variables|Default|GetInitial%20Spot) false true))

(event Custom|FlagDrop
  (params (Location :type Vector)))

(event EventBeginPlay
  (Variables|Default|SetInitial%20Spot (Transformation|GetActorLocation self)))

(fn ConstructionScript)