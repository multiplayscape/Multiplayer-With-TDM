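; Elevator actor that raises its static mesh while a BP_FPS overlaps its sphere and lowers it when that overlap ends.
; A timeline played forward or in reverse lerps the mesh's relative Z between the height saved at BeginPlay and HeightEleator.
; The construction script uses PreviewMaxHeight to preview the raised position, otherwise placing the mesh at StartingHeight.
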(event OnComponentBeginOverlap(Sphere)
  (params (OverlappedComponent :type Primitive%20Component%20Object%20Reference) (OtherActor :type Actor%20Object%20Reference) (OtherComp :type Primitive%20Component%20Object%20Reference) (OtherBodyIndex :type Integer) (bFromSweep :type Boolean) (SweepResult :type Hit%20Result%20Structure%20%28by%20ref%29))
  (Utilities|Casting|CastToBP_FPS OtherActor)
  (CallFunction|LiftUp))

(event OnComponentEndOverlap(Sphere)
  (params (OverlappedComponent :type Primitive%20Component%20Object%20Reference) (OtherActor :type Actor%20Object%20Reference) (OtherComp :type Primitive%20Component%20Object%20Reference) (OtherBodyIndex :type Integer))
  (Utilities|Casting|CastToBP_FPS OtherActor)
  (CallFunction|LiftDown))

(event Custom|Lift%20Down
  (bind _staticmesh (Variables|Default|GetStaticMesh))
  (bind _relativelocation (Variables|/Script/Engine.SceneComponent|GetRelativeLocation _staticmesh))
  (bind _newtrack_0 (Timeline|Timeline_0 Reverse)
    (:Update
      (Transformation|SetRelativeLocation _staticmesh (Math|Vector|MakeVector (.x _relativelocation) (.y _relativelocation) (Math|Float|Lerp (Variables|Default|GetstartingHeight) (Variables|Default|GetheightEleator) _newtrack_0)) false false))))

(event Custom|Lift%20up
  (bind _staticmesh (Variables|Default|GetStaticMesh))
  (bind _relativelocation (Variables|/Script/Engine.SceneComponent|GetRelativeLocation _staticmesh))
  (bind _newtrack_0 (Timeline|Timeline_0 Play)
    (:Update
      (Transformation|SetRelativeLocation _staticmesh (Math|Vector|MakeVector (.x _relativelocation) (.y _relativelocation) (Math|Float|Lerp (Variables|Default|GetstartingHeight) (Variables|Default|GetheightEleator) _newtrack_0)) false false))))

(event EventBeginPlay
  (Variables|Default|SetstartingHeight (.z (Variables|/Script/Engine.SceneComponent|GetRelativeLocation (Variables|Default|GetStaticMesh)))))

(fn ConstructionScript
  (bind _staticmesh (Variables|Default|GetStaticMesh))
  (bind _relativelocation (Variables|/Script/Engine.SceneComponent|GetRelativeLocation _staticmesh))
  (if (Variables|Default|GetpreviewMaxHeight)
    (Variables|Default|SetdevHeight (.z _relativelocation))
    (Transformation|SetRelativeLocation _staticmesh (Math|Vector|MakeVector (.x _relativelocation) (.y _relativelocation) (Variables|Default|GetheightEleator)) false false)
    (else
      (Transformation|SetRelativeLocation _staticmesh (Math|Vector|MakeVector (.x _relativelocation) (.y _relativelocation) (Variables|Default|GetstartingHeight)) false false))))