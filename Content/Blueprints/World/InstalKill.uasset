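; InstalKill is a world actor with a rotating orb that deals likely lethal point damage to a BP_FPS player who touches it.
; Tick spins the Orb around its yaw axis at a steady rate.
; While OrbAvailable is true, any overlap hides the orb, then a BP_FPS cast gates the damage.
; The graph never clears OrbAvailable, so hiding the orb does not disarm it.
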(event OnComponentBeginOverlap(Orb)
  (params (OverlappedComponent :type Primitive%20Component%20Object%20Reference) (OtherActor :type Actor%20Object%20Reference) (OtherComp :type Primitive%20Component%20Object%20Reference) (OtherBodyIndex :type Integer) (bFromSweep :type Boolean) (SweepResult :type Hit%20Result%20Structure%20%28by%20ref%29))
  (if (Variables|Default|GetOrbAvailable)
    (Rendering|SetVisibility (Variables|Default|GetOrb) false false)
    (bind _asbp_fps (Utilities|Casting|CastToBP_FPS OtherActor))
    (Game|Damage|ApplyPointDamage _asbp_fps 1e+03 (Math|Vector|MakeVector 0.0 0.0 0.0) (Collision|MakeHitResult false false 0.0 0.0 "0, 0, 0" "0, 0, 0" "0,0,1" "0,0,1" 0 0))))

(event EventBeginPlay)

(event EventTick
  (params (DeltaSeconds :type Float%20%28single-precision%29))
  (Transformation|AddWorldRotation (Variables|Default|GetOrb) (Math|Rotator|MakeRotator 0.0 0.0 (* DeltaSeconds 24.0)) false false))

(fn ConstructionScript)