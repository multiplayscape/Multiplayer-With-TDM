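; Health pickup orb that restores HP to a BP_FPS character on overlap and respawns after a short delay.
; Overlap hides the Orb component, adds health clamped to a fixed range, and uses an availability flag and Delay to block pickup until it reappears.
; The orb hides before the cast, so other overlapping actors leave it invisible but still available.
; Tick spins the orb around yaw at a frame-rate-independent speed.
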(event OnComponentBeginOverlap(Orb)
  (params (OverlappedComponent :type Primitive%20Component%20Object%20Reference) (OtherActor :type Actor%20Object%20Reference) (OtherComp :type Primitive%20Component%20Object%20Reference) (OtherBodyIndex :type Integer) (bFromSweep :type Boolean) (SweepResult :type Hit%20Result%20Structure%20%28by%20ref%29))
  (if (Variables|Default|GetOrbAvailable)
    (Rendering|SetVisibility (Variables|Default|GetOrb) false false)
    (bind _asbp_fps (Utilities|Casting|CastToBP_FPS OtherActor))
    (Variables|/Game/Blueprints/Characters/BP_FPS.BP_FPS_C|SetHPCurrent _asbp_fps (Math|Float|Clamp(Float) (+ (Variables|/Game/Blueprints/Characters/BP_FPS.BP_FPS_C|GetHPCurrent _asbp_fps) 5e+01) 0.0 2e+02))
    (Variables|Default|SetOrbAvailable false)
    (Utilities|FlowControl|Delay 1e+01)
    (Variables|Default|SetOrbAvailable true)
    (Rendering|SetVisibility (Variables|Default|GetOrb) true false)))

(event EventBeginPlay)

(event EventTick
  (params (DeltaSeconds :type Float%20%28single-precision%29))
  (Transformation|AddWorldRotation (Variables|Default|GetOrb) (Math|Rotator|MakeRotator 0.0 0.0 (* DeltaSeconds 24.0)) false false))

(fn ConstructionScript)