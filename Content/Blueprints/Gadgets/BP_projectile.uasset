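; Gadget projectile, such as a grenade, that spawns a detonation effect actor at its transform and destroys itself when a fuse timer expires.
; Its construction script reads the Gadget row from GadgetTable to set fuse time, effect class, bounce limit, bounciness, mesh and scale.
; Bounces increment a hit counter and switch off rotation-follows-velocity while the count is below the limit; reaching the limit does not trigger detonation.
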(event OnProjectileBounce(ProjectileMovement)
  (params (ImpactResult :type Hit%20Result%20Structure%20%28by%20ref%29) (ImpactVelocity :type Vector%20%28by%20ref%29 :default "0, 0, 0"))
  (bind _indexhit (Variables|Default|GetindexHit))
  (Math|Integer|IncrementInt _indexhit
    (:%20%20
      (if (< _indexhit (Variables|Default|GetnumberBounce))
        (Variables|/Script/Engine.ProjectileMovementComponent|SetbRotationFollowsVelocity (Variables|Default|GetProjectileMovement) false)))))

(event Custom|Detonate
  (bind _returnvalue (Transformation|GetActorTransform))
  (Game|SpawnActorfromClass (Variables|Default|GeteffectOnDetonate) (Math|Transform|MakeTransform (.location _returnvalue) (.rotation _returnvalue) (.scale _returnvalue)) "AlwaysSpawn" 0 0)
  (Actor|DestroyActor))

(event EventBeginPlay
  (Utilities|Time|SetTimerbyEvent (delegate Custom|Detonate) (Variables|Default|GettimeLimit)))

(fn ConstructionScript
  (bind _grenademesh (Variables|Default|GetGrenadeMesh))
  (bind _returnvalue (Utilities|GetDataTableRow "/Game/Blueprints/Tables/gadgetTable.gadgetTable" (Variables|Default|Getgadget))
    (:then
      (Variables|Default|SettimeLimit (.timeBeforeDetonate (Utilities|Struct|BreakgadgetStruct _returnvalue)))
      (Variables|Default|SeteffectOnDetonate (.effectOnDetonate (Utilities|Struct|BreakgadgetStruct _returnvalue)))
      (Variables|Default|SetnumberBounce (.maxBounce (Utilities|Struct|BreakgadgetStruct _returnvalue)))
      (Variables|/Script/Engine.ProjectileMovementComponent|SetBounciness (Variables|Default|GetProjectileMovement) (.bounciness (Utilities|Struct|BreakgadgetStruct _returnvalue)))
      (Components|StaticMesh|SetStaticMesh _grenademesh (.mesh (Utilities|Struct|BreakgadgetStruct _returnvalue)))
      (Transformation|SetWorldScale3D _grenademesh (.scaleMesh (Utilities|Struct|BreakgadgetStruct _returnvalue))))))