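; Master weapon Blueprint that handles the visual magazine swap on non-authority instances only.
; Its events turn on physics for the current magazine, then create a replacement component with the same mesh on the pawn's magazine socket.
; The replacement attaches to the first-person arms when locally controlled or the body mesh otherwise.
; A final event moves it onto the pawn's primary weapon mesh.
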(event Custom|removeMagazine
  (Networking|SwitchHasAuthority
    (:Remote
      (Physics|SetSimulatePhysics (Variables|Default|GetmagazineFPS) true))))

(event Custom|spawnNewMagazine
  (bind _pawn (Variables|Default|Getpawn))
  (Networking|SwitchHasAuthority
    (:Remote
      (bind _returnvalue (AddComponent|AddStaticMeshComponent true (Math|Transform|MakeTransform "0, 0, 0")))
      (Components|StaticMesh|SetStaticMesh _returnvalue (Variables|/Script/Engine.StaticMeshComponent|GetStaticMesh (Variables|Default|GetmagazineFPS)))
      (Variables|Default|SetmagazineFPS _returnvalue)
      (if (Pawn|IsLocallyControlled _pawn)
        (Transformation|AttachComponentToComponent (Variables|Default|GetmagazineFPS) (Variables|/Game/Blueprints/Characters/BP_FPS.BP_FPS_C|GetArms _pawn) "magazine" "SnapToTarget" "SnapToTarget" "KeepRelative" true)
        (else
          (Transformation|AttachComponentToComponent (Variables|Default|GetmagazineFPS) (Variables|/Script/Engine.Character|GetMesh _pawn) "magazine" "SnapToTarget" "SnapToTarget" "KeepRelative" true))))))

(event Custom|attachNewMagazine
  (bind _magazinefps (Variables|Default|GetmagazineFPS))
  (Networking|SwitchHasAuthority
    (:Remote
      (Transformation|DetachFromComponent _magazinefps "KeepRelative" "KeepRelative" "KeepRelative" true)
      (Transformation|AttachComponentToComponent _magazinefps (Variables|_WeaponMaster_C|GetWeaponMesh (Variables|/Game/Blueprints/Characters/BP_FPS.BP_FPS_C|GetPrimaryWeaponRef (Variables|Default|Getpawn))) "magazine" "SnapToTarget" "SnapToTarget" "KeepRelative" true))))

(fn ConstructionScript)