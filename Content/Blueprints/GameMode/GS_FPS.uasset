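; GS_FPS, apparently the game state for an FPS mode, holds the countdown for an initialization phase and a game phase.
; Each phase's start event seeds Seconds and starts a looping one-second timer that decrements it through TimerDisplay.
; The initialization event also records its starting duration, while the game event sets GameReady.
; Both store the handle in GameTimer, and nothing here clears the timer or stops at zero.
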(event Custom|TimerInitializeTick
  (params (Seconds :type Float%20%28single-precision%29))
  (bind _output_get (Variables|Default|SetSeconds Seconds))
  (Variables|Default|SetgameIniSeconds _output_get)
  (bind _returnvalue (Utilities|Time|SetTimerbyEvent (delegate Custom|TimerDisplay) 1.0 true))
  (Variables|Default|SetGameTimer _returnvalue))

(event Custom|TimerGameTick
  (params (Seconds :type Float%20%28single-precision%29))
  (Variables|Default|SetgameReady true)
  (Variables|Default|SetSeconds Seconds)
  (bind _returnvalue (Utilities|Time|SetTimerbyEvent (delegate Custom|TimerDisplay) 1.0 true))
  (Variables|Default|SetGameTimer _returnvalue))

(event Custom|TimerDisplay
  (Math|Float|DecrementFloat (Variables|Default|GetSeconds)))

(fn ConstructionScript)