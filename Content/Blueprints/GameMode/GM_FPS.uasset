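; Server game mode for the multiplayer FPS that runs FFA and team deathmatch matches and registers with GameLift.
; A full lobby starts prepare and match timers from per-mode settings, then time-up freezes players and picks winners or draws by kills.
; Tagged PlayerStarts feed team or random spawns, and kill feed and scores relay through controllers or pawns.
; TDM logouts spawn an invulnerable stand-in pawn carrying the leaver's stats.
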(event Custom|FinishGame
  ;[1 0.2717 0] Finish Game (On Time's up, or Winning Condition)
  (CallFunction|GameOverAllPlayers)
  (switch Utilities|FlowControl|Switch|SwitchonGamemodes (Variables|Default|GetMode)
    (:NewEnumerator0
      (CallFunction|FFAending))
    (:NewEnumerator1
      (CallFunction|TDMending))))

(event Custom|PlatformCall
  (params (Obj :type Array%20of%20Platform%20Object%20References))
  ;[1 0.9201 0] Platform - Ensure Replication
  (Utilities|FlowControl|Delay 1.0)
  (for _array_element Obj
    (Default|Start _array_element))
  (for _array_element_2 (Variables|Default|GetControllerArray)
    (bind _aspc_fps (Utilities|Casting|CastToPC_FPS _array_element_2))
    (Default|PlatformCallonPC _aspc_fps Obj)))

(event Custom|GameliftRequired
  ;[0.008 0 0.992] Post-login | Begin Play | Set Respawn points & Controllers | Timer Management
  (if (Networking|IsServer)
    (bind (_success _errortype _errormessage) (Class|GameLiftServerFunctionLibrary|InitSDK))
    (if _success
      (bind _returnvalue (Game|ConstructObjectfromClass "/Game/FirstPersonBP/Blueprints/ProcessParametersEx.ProcessParametersEx_C" self (.port (Class|ServerHelper|ServerIPandPort)) (Utilities|Array|MakeArray "../../Saved/Logs")))
      (bind (_success_2 _errortype_2 _errormessage_2) (Class|GameLiftServerFunctionLibrary|ProcessReady _returnvalue))
      (if (not _success_2)
        (Development|PrintString _errormessage_2))
      (else
        (Development|PrintString _errormessage)))))

(event Custom|TimeUp
  ;[0.008 0 0.992] Post-login | Begin Play | Set Respawn points & Controllers | Timer Management
  (CallFunction|FinishGame)
  (Utilities|Time|ClearandInvalidateTimerbyHandle (stale Custom|gameStart _returnvalue))
  (Utilities|Time|ClearandInvalidateTimerbyHandle (Variables|/Game/Blueprints/GameMode/GS_FPS.GS_FPS_C|GetGameTimer (stale Custom|gameStart _asgs_fps)))
  (for _array_element (Variables|Default|GetControllerArray)
    (Class|GameplayStatics|RemovePlayer _array_element true) ; Doesn't Work
  ))

(event Custom|gameStart
  (bind _gamemodesettings (Variables|Default|GetgameModeSettings))
  (bind _mode (Variables|Default|GetMode))
  (bind _value (Utilities|Map|Find _gamemodesettings _mode))
  (bind _timelimit (Utilities|Struct|BreakGameModeSettingsStruct _value))
  ;[0.008 0 0.992] Post-login | Begin Play | Set Respawn points & Controllers | Timer Management
  (Utilities|FlowControl|Delay 0.2)
  (Variables|Default|SetisGameStart true)
  (CallFunction|InitializedAllPlayers)
  (bind _asgs_fps (Utilities|Casting|CastToGS_FPS (Game|GetGameState)))
  (Default|TimerGameTick _asgs_fps _timelimit)
  (bind _returnvalue (Utilities|Time|SetTimerbyEvent (delegate Custom|TimeUp) _timelimit)))

(event Custom|initializedAllPlayers
  ;[0.008 0 0.992] Post-login | Begin Play | Set Respawn points & Controllers | Timer Management
  (for _array_element (Variables|Default|GetControllerArray)
    (bind _aspc_fps (Utilities|Casting|CastToPC_FPS _array_element))
    (Default|GameReady _aspc_fps)
    (if (Variables|/Game/Blueprints/Characters/PC_FPS.PC_FPS_C|GetisReady _aspc_fps)
      (Utilities|IsValid (Variables|/Game/Blueprints/Characters/PC_FPS.PC_FPS_C|GetpawnRef _aspc_fps)
        (:Is%20Valid
          (Variables|/Game/Blueprints/Characters/BP_FPS.BP_FPS_C|SetcanThrow (Variables|/Game/Blueprints/Characters/PC_FPS.PC_FPS_C|GetpawnRef _aspc_fps) true)
          (Variables|/Game/Blueprints/Characters/BP_FPS.BP_FPS_C|SetCanShoot (Variables|/Game/Blueprints/Characters/PC_FPS.PC_FPS_C|GetpawnRef _aspc_fps) true)
          (Pawn|Components|CharacterMovement|SetMovementMode (Variables|/Script/Engine.Character|GetCharacterMovement (Variables|/Game/Blueprints/Characters/PC_FPS.PC_FPS_C|GetpawnRef _aspc_fps)) "MOVE_Walking" 0)
          (Variables|/Script/Engine.CharacterMovementComponent|SetDefaultLandMovementMode (Variables|/Script/Engine.Character|GetCharacterMovement (Variables|/Game/Blueprints/Characters/PC_FPS.PC_FPS_C|GetpawnRef _aspc_fps)) "MOVE_Walking"))))))

(event Custom|gameOverAllPlayers
  ;[0.008 0 0.992] Post-login | Begin Play | Set Respawn points & Controllers | Timer Management
  (for _array_element (Variables|Default|GetControllerArray)
    (bind _aspc_fps (Utilities|Casting|CastToPC_FPS _array_element))
    (Default|GameOver _aspc_fps)
    (Utilities|IsValid (Variables|/Game/Blueprints/Characters/PC_FPS.PC_FPS_C|GetpawnRef _aspc_fps)
      (:Is%20Valid
        (Variables|/Game/Blueprints/Characters/BP_FPS.BP_FPS_C|SetcanThrow (Variables|/Game/Blueprints/Characters/PC_FPS.PC_FPS_C|GetpawnRef _aspc_fps) false)
        (Variables|/Game/Blueprints/Characters/BP_FPS.BP_FPS_C|SetCanShoot (Variables|/Game/Blueprints/Characters/PC_FPS.PC_FPS_C|GetpawnRef _aspc_fps) false)
        (if (AI|Components|NavMovement|IsFalling (Variables|/Script/Engine.Character|GetCharacterMovement (Variables|/Game/Blueprints/Characters/PC_FPS.PC_FPS_C|GetpawnRef _aspc_fps)))
          (Pawn|Components|CharacterMovement|SetMovementMode (Variables|/Script/Engine.Character|GetCharacterMovement (Variables|/Game/Blueprints/Characters/PC_FPS.PC_FPS_C|GetpawnRef _aspc_fps)) "MOVE_Falling" 0)
          (else
            (Pawn|Components|CharacterMovement|SetMovementMode (Variables|/Script/Engine.Character|GetCharacterMovement (Variables|/Game/Blueprints/Characters/PC_FPS.PC_FPS_C|GetpawnRef _aspc_fps)) "MOVE_None" 0)))
        (Variables|/Script/Engine.CharacterMovementComponent|SetDefaultLandMovementMode (Variables|/Script/Engine.Character|GetCharacterMovement (Variables|/Game/Blueprints/Characters/PC_FPS.PC_FPS_C|GetpawnRef _aspc_fps)) "MOVE_None")))))

(event Custom|ServerKillFeed
  (params (KilledPlayer :type String) (KillerTeam :type Teams%20Enum :default "NewEnumerator0") (KilledTeam :type Teams%20Enum :default "NewEnumerator0"))
  ;[1 0 0.7435] Populate Killfeed for every active player
  (for _array_element (Variables|Default|GetControllerArray)
    (bind _asbp_fps (Utilities|Casting|CastToBP_FPS (Pawn|GetControlledPawn _array_element)))
    (Default|PopulateKillFeed _asbp_fps 0 KilledPlayer KillerTeam KilledTeam)))

(event Custom|updateQuickScoreboard
  (params (team :type Teams%20Enum :default "NewEnumerator0") (pawn :type BP%20FPS%20Object%20Reference) (score :type Integer))
  (bind _controllerarray (Variables|Default|GetControllerArray))
  (switch Utilities|FlowControl|Switch|SwitchonGamemodes (Variables|Default|GetMode)
    (:NewEnumerator0
      (for _array_element _controllerarray
        (bind _aspc_fps (Utilities|Casting|CastToPC_FPS _array_element))
        (Utilities|IsValid (Variables|/Game/Blueprints/Characters/PC_FPS.PC_FPS_C|GetpawnRef _aspc_fps)
          (:Is%20Valid
            (Default|UpdateQuickScoreboardCall _aspc_fps (== (Variables|/Game/Blueprints/Characters/PC_FPS.PC_FPS_C|GetpawnRef _aspc_fps) pawn) "NewEnumerator0" score))
          (:Is%20Not%20Valid
            (Default|UpdateQuickScoreboardCall _aspc_fps false "NewEnumerator0" score)))))
    (:NewEnumerator1
      (for _array_element_2 _controllerarray
        (bind _aspc_fps_2 (Utilities|Casting|CastToPC_FPS _array_element_2))
        (Default|UpdateQuickScoreboardCall _aspc_fps_2 false team)
        (Default|UpdateScoreboardCall _aspc_fps_2 team)))))

(event EventPostLogin
  (params (NewPlayer :type Player%20Controller%20Object%20Reference))
  (bind _controllerarray (Variables|Default|GetControllerArray))
  (bind _gamemodesettings (Variables|Default|GetgameModeSettings))
  (bind _mode (Variables|Default|GetMode))
  (bind _value (Utilities|Map|Find _gamemodesettings _mode))
  (bind _timeprepare (Utilities|Struct|BreakGameModeSettingsStruct _value))
  ;[0.008 0 0.992] Post-login | Begin Play | Set Respawn points & Controllers | Timer Management
  (bind _aspc_fps (Utilities|Casting|CastToPC_FPS NewPlayer))
  (Utilities|Array|Add _controllerarray _aspc_fps)
  (if (not (< (Utilities|Array|Length _controllerarray) (Variables|Default|GetMaxPlayers)))
    (bind _asgs_fps (Utilities|Casting|CastToGS_FPS (Game|GetGameState)))
    (Default|TimerInitializeTick _asgs_fps _timeprepare)
    (Utilities|Time|SetTimerbyEvent (delegate Custom|gameStart) _timeprepare)))

(event EventBeginPlay
  ;[0.008 0 0.992] Post-login | Begin Play | Set Respawn points & Controllers | Timer Management
  (|CallParentFunction)
  (CallFunction|GameliftRequired)
  (bind _outactors (Actor|GetAllActorsOfClass "/Script/Engine.PlayerStart"))
  (bind _output_get (Variables|Default|SetRespawnPoints _outactors))
  (for _array_element _output_get
    (if (Utilities|Name|Equal(Name) (Utilities|Array|Get(acopy) (Variables|/Script/Engine.Actor|GetTags _array_element)) "team1")
      (Utilities|Array|Add (Variables|Default|GetRespawnPointTeam1) _array_element)
      (elif (Utilities|Name|Equal(Name) (Utilities|Array|Get(acopy) (Variables|/Script/Engine.Actor|GetTags _array_element)) "random")
        (Utilities|Array|Add (Variables|Default|GetRespawnPointRandom) _array_element)
        (else
          (Utilities|Array|Add (Variables|Default|GetRespawnPointTeam2) _array_element)))))
  (switch Utilities|FlowControl|Switch|SwitchonGamemodes (Variables|Default|GetMode)))

(event EventOnLogout
  (params (ExitingController :type Controller%20Object%20Reference))
  ;[0.008 0 0.992] Post-login | Begin Play | Set Respawn points & Controllers | Timer Management
  (switch Utilities|FlowControl|Switch|SwitchonGamemodes (Variables|Default|GetMode)
    (:NewEnumerator0
      (bind _aspc_fps (Utilities|Casting|CastToPC_FPS ExitingController))
      (Class|GameplayStatics|RemovePlayer _aspc_fps true))
    (:NewEnumerator1
      (bind _aspc_fps_2 (Utilities|Casting|CastToPC_FPS ExitingController))
      (CallFunction|UnpopulateTeam (Variables|/Game/Blueprints/Characters/PC_FPS.PC_FPS_C|GetTeam _aspc_fps_2) (Variables|/Game/Blueprints/Characters/PC_FPS.PC_FPS_C|GetpawnRef _aspc_fps_2))
      (bind _returnvalue (Game|SpawnActorfromClass "/Game/Blueprints/Characters/BP_FPS.BP_FPS_C" (Math|Transform|MakeTransform "-5310.000000,-1770.000000,500.000000" "0, 0, 0" "1,1,1") "AlwaysSpawn" 0 false (Variables|/Game/Blueprints/Characters/PC_FPS.PC_FPS_C|GetTeam _aspc_fps_2) "NewEnumerator0" false (Variables|/Game/Blueprints/Characters/BP_FPS.BP_FPS_C|GetPlayerStats (Variables|/Game/Blueprints/Characters/PC_FPS.PC_FPS_C|GetpawnRef _aspc_fps_2)) (Variables|/Game/Blueprints/Characters/PC_FPS.PC_FPS_C|GetPlayerName _aspc_fps_2) 0))
      (Variables|/Script/Engine.Actor|SetbCanBeDamaged _returnvalue false)
      (CallFunction|PopulateTeam (Variables|/Game/Blueprints/Characters/PC_FPS.PC_FPS_C|GetTeam _aspc_fps_2) _returnvalue))))

(event EventTick
  (params (DeltaSeconds :type Float%20%28single-precision%29)))

(fn ConstructionScript)

(fn SpawnTeamSelect
  (params (TeamSelected :type Teams%20Enum :default "NewEnumerator0") (gunType :type gunTypeEnum%20Enum :default "NewEnumerator0") (controller :type PC%20FPS%20Object%20Reference) (pawn :type BP%20FPS%20Object%20Reference%20%28by%20ref%29))
  (bind _pawnarray (LocalVariables|GetpawnArray))
  (bind _charactermovement (Variables|/Script/Engine.Character|GetCharacterMovement pawn))
  (bind _respawnpointrandom (Variables|Default|GetRespawnPointRandom))
  (bind _respawnpointteam1 (Variables|Default|GetRespawnPointTeam1))
  (bind _respawnpointteam2 (Variables|Default|GetRespawnPointTeam2))
  (bind _mode (Variables|Default|GetMode))
  (bind _team (Variables|Default|Getteam))
  (bind _returnvalue (Utilities|Array|Length _respawnpointrandom))
  (bind _returnvalue_2 (Utilities|Array|Length _respawnpointteam2))
  (bind _returnvalue_3 (Utilities|Array|Length _respawnpointteam1))
  (bind _value (Utilities|Map|Find _team TeamSelected))
  (bind _returnvalue_4 (- _returnvalue_2 1))
  (bind _returnvalue_5 (- _returnvalue 1))
  (bind _returnvalue_6 (- _returnvalue_3 1))
  (bind _returnvalue_7 (Math|Random|RandomIntegerinRange 0 _returnvalue_5))
  (bind _returnvalue_8 (Math|Random|RandomIntegerinRange 0 _returnvalue_6))
  (bind _returnvalue_9 (Math|Random|RandomIntegerinRange 0 _returnvalue_4))
  (bind _output (Utilities|Array|Get(acopy) _respawnpointteam2 _returnvalue_9))
  (bind _output_2 (Utilities|Array|Get(acopy) _respawnpointrandom _returnvalue_7))
  (bind _output_3 (Utilities|Array|Get(acopy) _respawnpointteam1 _returnvalue_8))
  (bind _returnvalue_10 (Utilities|Select :Index TeamSelected :NewEnumerator0 _output_2 :NewEnumerator1 _output_3 :NewEnumerator2 _output))
  (bind _returnvalue_11 (Utilities|Select :Index _mode :NewEnumerator0 _output_2 :NewEnumerator1 _returnvalue_10 :NewEnumerator2 0 :NewEnumerator3 0 :NewEnumerator4 0))
  (bind _returnvalue_12 (Transformation|GetActorTransform _returnvalue_11))
  (Transformation|SetActorTransform pawn (Math|Transform|MakeTransform (.location _returnvalue_12) (.rotation _returnvalue_12)))
  (Utilities|Array|Add _pawnarray pawn)
  (Utilities|Array|AppendArray _pawnarray (Utilities|Struct|BreakteamArrayStruct _value))
  (bind _structout (Utilities|Struct|SetmembersinteamArrayStruct _value _pawnarray))
  (Utilities|Map|Add _team TeamSelected _structout)
  (if (Variables|Default|GetisGameStart)
    (Pawn|Components|CharacterMovement|SetMovementMode _charactermovement "MOVE_Walking" 0)
    (Variables|/Script/Engine.CharacterMovementComponent|SetDefaultLandMovementMode _charactermovement "MOVE_Walking")
    (Variables|/Game/Blueprints/Characters/BP_FPS.BP_FPS_C|SetcanThrow pawn true)
    (Variables|/Game/Blueprints/Characters/BP_FPS.BP_FPS_C|SetCanShoot pawn true))
  (LocalVariables|SetpawnRef pawn)
  (Utilities|Array|AddUnique (Variables|/Game/Blueprints/GameMode/GS_FPS.GS_FPS_C|GetPlayers (.AsGS%20FPS (Utilities|Casting|CastToGS_FPS (Game|GetGameState)))) pawn)
  (Default|SetWidgetPawnRef controller pawn TeamSelected)
  (return (LocalVariables|GetpawnRef)))

(fn FFAending
  (for _array_element (Variables|Default|GetControllerArray)
    (bind _aspc_fps (Utilities|Casting|CastToPC_FPS _array_element))
    (Utilities|IsValid (Variables|/Game/Blueprints/Characters/PC_FPS.PC_FPS_C|GetpawnRef _aspc_fps)
      (:Is%20Valid
        (if (> (.Kills (Utilities|Struct|BreakPlayerStats (Variables|/Game/Blueprints/Characters/BP_FPS.BP_FPS_C|GetPlayerStats (Variables|/Game/Blueprints/Characters/PC_FPS.PC_FPS_C|GetpawnRef _aspc_fps)))) (.kills (Variables|Default|GetWinnerStats)))
          (Variables|Default|SetWinnerStats (Variables|/Game/Blueprints/Characters/BP_FPS.BP_FPS_C|GetPlayerStats (Variables|/Game/Blueprints/Characters/PC_FPS.PC_FPS_C|GetpawnRef _aspc_fps)))
          (Variables|Default|SetWinner _aspc_fps)
          (Utilities|Array|Clear (Variables|Default|GetDrawArray)) ; If a new "Winner" has a better score than everyone else. Clear the array.
          (elif (== (.Kills (Utilities|Struct|BreakPlayerStats (Variables|/Game/Blueprints/Characters/BP_FPS.BP_FPS_C|GetPlayerStats (Variables|/Game/Blueprints/Characters/PC_FPS.PC_FPS_C|GetpawnRef _aspc_fps)))) (.kills (Variables|Default|GetWinnerStats)))
            (Utilities|Array|Add (Variables|Default|GetDrawArray) _aspc_fps) ; Array of players with the same Best Score
          )))))
  (if (> (Utilities|Array|Length (Variables|Default|GetDrawArray)) 0) ; If there's a Draw
    (for _array_element_2 (Variables|Default|GetDrawArray)
      (bind _aspc_fps_2 (Utilities|Casting|CastToPC_FPS _array_element_2))
      (Default|WinningServer _aspc_fps_2 (Variables|/Game/Blueprints/Characters/PC_FPS.PC_FPS_C|GetPlayerName _aspc_fps_2) true))
    (Utilities|IsValid (Variables|Default|GetWinner)
      (:Is%20Valid
        (Default|WinningServer (Variables|Default|GetWinner) (Variables|/Game/Blueprints/Characters/PC_FPS.PC_FPS_C|GetPlayerName (Variables|Default|GetWinner)) true))
      (:Is%20Not%20Valid
        _))
    (for _array_element_3 (Variables|Default|GetControllerArray) ; Everyone else Loses
      (bind _aspc_fps_3 (Utilities|Casting|CastToPC_FPS _array_element_3))
      (if (not (Utilities|Array|ContainsItem (Variables|Default|GetDrawArray) _aspc_fps_3))
        (Default|LosingServer _aspc_fps_3 (Variables|/Game/Blueprints/Characters/PC_FPS.PC_FPS_C|GetPlayerName _aspc_fps_3))))
    (else
      (for _array_element_4 (Variables|Default|GetControllerArray)
        (if (not (== _array_element_4 (Variables|Default|GetWinner)))
          (bind _aspc_fps_4 (Utilities|Casting|CastToPC_FPS _array_element_4))
          (Default|LosingServer _aspc_fps_4 (Variables|/Game/Blueprints/Characters/PC_FPS.PC_FPS_C|GetPlayerName _aspc_fps_4))))
      (Utilities|IsValid (Variables|Default|GetWinner)
        (:Is%20Valid
          (Default|WinningServer (Variables|Default|GetWinner) (Variables|/Game/Blueprints/Characters/PC_FPS.PC_FPS_C|GetPlayerName (Variables|Default|GetWinner)) false))))))

(fn TDMending
  (bind _team (Variables|Default|Getteam))
  (bind _teamscore (LocalVariables|GetteamScore))
  (bind _teamscore_2 (LocalVariables|GetteamScore))
  (bind _value (Utilities|Map|Find _teamscore_2 "NewEnumerator1"))
  (bind _value_2 (Utilities|Map|Find _teamscore_2 "NewEnumerator2"))
  (bind _keys (Utilities|Map|Keys _team))
  (for _array_element _keys
    (for _array_element_2 (.pawn (.Value (Utilities|Map|Find _team _array_element)))
      (Utilities|Map|Add _teamscore _array_element (+ (.Value (Utilities|Map|Find _teamscore _array_element)) (.kills (Variables|/Game/Blueprints/Characters/BP_FPS.BP_FPS_C|GetPlayerStats _array_element_2))))))
  (if (== _value _value_2)
    (for _array_element_3 (Variables|Default|GetControllerArray)
      (bind _aspc_fps (Utilities|Casting|CastToPC_FPS _array_element_3))
      (Default|WinningServer _aspc_fps (Variables|/Game/Blueprints/Characters/PC_FPS.PC_FPS_C|GetPlayerName _aspc_fps) true))
    (elif (< _value _value_2)
      (for _array_element_4 (Variables|Default|GetControllerArray)
        (bind _aspc_fps_2 (Utilities|Casting|CastToPC_FPS _array_element_4))
        (if (Utilities|Enum|Equal(Enum) (Variables|/Game/Blueprints/Characters/BP_FPS.BP_FPS_C|GetTeam (Variables|/Game/Blueprints/Characters/PC_FPS.PC_FPS_C|GetpawnRef _aspc_fps_2)) "NewEnumerator2")
          (Default|WinningServer _aspc_fps_2 (Variables|/Game/Blueprints/Characters/PC_FPS.PC_FPS_C|GetPlayerName _aspc_fps_2) false)
          (else
            (Default|LosingServer _aspc_fps_2 (Variables|/Game/Blueprints/Characters/PC_FPS.PC_FPS_C|GetPlayerName _aspc_fps_2)))))
      (else
        (for _array_element_5 (Variables|Default|GetControllerArray)
          (bind _aspc_fps_3 (Utilities|Casting|CastToPC_FPS _array_element_5))
          (if (Utilities|Enum|Equal(Enum) (Variables|/Game/Blueprints/Characters/BP_FPS.BP_FPS_C|GetTeam (Variables|/Game/Blueprints/Characters/PC_FPS.PC_FPS_C|GetpawnRef _aspc_fps_3)) "NewEnumerator1")
            (Default|WinningServer _aspc_fps_3 (Variables|/Game/Blueprints/Characters/PC_FPS.PC_FPS_C|GetPlayerName _aspc_fps_3) false)
            (else
              (Default|LosingServer _aspc_fps_3 (Variables|/Game/Blueprints/Characters/PC_FPS.PC_FPS_C|GetPlayerName _aspc_fps_3)))))))))

(fn UnpopulateTeam
  (params (Team :type Teams%20Enum%20%28by%20ref%29 :default "NewEnumerator0") (Pawn :type BP%20FPS%20Object%20Reference%20%28by%20ref%29))
  (bind _team (Variables|Default|Getteam))
  (bind _output_get (LocalVariables|SetTeamTMP (.pawn (.Value (Utilities|Map|Find _team Team)))))
  (Utilities|Array|RemoveItem _output_get Pawn)
  (Utilities|Map|Add _team Team (Utilities|Struct|MaketeamArrayStruct (LocalVariables|GetTeamTMP)))
  (return))

(fn PopulateTeam
  (params (Team :type Teams%20Enum%20%28by%20ref%29 :default "NewEnumerator0") (Pawn :type BP%20FPS%20Object%20Reference%20%28by%20ref%29))
  (bind _team (Variables|Default|Getteam))
  (bind _output_get (LocalVariables|SetTeamTMP (.pawn (.Value (Utilities|Map|Find _team Team)))))
  (Utilities|Array|Add _output_get Pawn)
  (Utilities|Map|Add _team Team (Utilities|Struct|MaketeamArrayStruct (LocalVariables|GetTeamTMP))))