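; HUD class for the FPS game that creates and controls the player's on-screen widgets.
; BeginPlay adds the main HUD and timer; the scoreboard is built on request per game mode, and the respawn screen on first display.
; Events forward ammo and hit markers to the main widget and toggle visibility of player info, scoreboard and respawn screen.
; It also adds team-colored killfeed entries and opens chat in team or global mode.
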(event Custom|HideHUD
  (bind _hudwidgetref (Variables|Default|GetHUDWidgetREF))
  ;[0.2204 0 1] Show // Hide {W_HUD}
  (Utilities|IsValid _hudwidgetref
    (:Is%20Valid
      (Widget|SetVisibility (Variables|/Game/UMG/Widgets/W_HUD.W_HUD_C|GetPlayerInfos _hudwidgetref) "Hidden"))))

(event Custom|DisplayHUD
  (bind _hudwidgetref (Variables|Default|GetHUDWidgetREF))
  ;[0.2204 0 1] Show // Hide {W_HUD}
  (Utilities|IsValid _hudwidgetref
    (:Is%20Valid
      (Widget|SetVisibility (Variables|/Game/UMG/Widgets/W_HUD.W_HUD_C|GetPlayerInfos _hudwidgetref) "Visible"))))

(event Custom|Hide%20Scoreboard
  ;[0.2204 0 1] Show // Hide {W_ScoreBoard}
  (Widget|SetVisibility (Variables|Default|GetScoreboardREF) "Hidden"))

(event Custom|createScoreBoard
  (params (isTeam :type Boolean) (gameMode :type Gamemodes%20Enum :default "NewEnumerator0"))
  ;[1 1 1] displayScoreboard
  (bind _returnvalue (UserInterface|CreateWidget "/Game/UMG/Widgets/W_ScoreBoard.W_ScoreBoard_C" 0 isTeam gameMode))
  (bind _output_get (Variables|Default|SetScoreboardREF _returnvalue))
  (UserInterface|Viewport|AddtoViewport _output_get 0))

(event Custom|DisplayKillFeed
  (params (KilledPlayer :type String) (Killer :type Teams%20Enum :default "NewEnumerator0") (Killed :type Teams%20Enum :default "NewEnumerator0"))
  ;[0.168 0 1] Show and populate Killfeed
  (bind _returnvalue (UserInterface|CreateWidget "/Game/UMG/Widgets/W_KillFeed.W_KillFeed_C" 0 KilledPlayer (Utilities|Struct|MakeSlateColor (Utilities|Select :Index Killer :NewEnumerator0 "(R=0.755208,G=0.755208,B=0.755208,A=1.000000)" :NewEnumerator1 "(R=0.000000,G=0.107611,B=1.000000,A=1.000000)" :NewEnumerator2 "(R=1.000000,G=0.018877,B=0.000000,A=1.000000)")) (Utilities|Struct|MakeSlateColor (Utilities|Select :Index Killed :NewEnumerator0 "(R=0.755208,G=0.755208,B=0.755208,A=1.000000)" :NewEnumerator1 "(R=0.000000,G=0.107611,B=1.000000,A=1.000000)" :NewEnumerator2 "(R=1.000000,G=0.018877,B=0.000000,A=1.000000)"))))
  (Widget|Panel|AddChild (Variables|/Game/UMG/Widgets/W_KillFeedContainer.W_KillFeedContainer_C|GetVerticalBoxKF (Variables|/Game/UMG/Widgets/W_HUD.W_HUD_C|GetW_KillFeedContainer (Variables|Default|GetHUDWidgetREF))) _returnvalue))

(event Custom|Display//Create%20Scoreboard
  (bind _scoreboardref (Variables|Default|GetScoreboardREF))
  ;[0.2204 0 1] Show // Hide {W_ScoreBoard}
  (Utilities|IsValid _scoreboardref
    (:Is%20Valid
      (Widget|SetVisibility _scoreboardref "Visible")
      (Default|RefreshList _scoreboardref))))

(event Custom|DisplayRespawnScreen
  ;[0.2204 0 1] Show // Hide {W_RespawnScreen}
  (Utilities|IsValid (Variables|Default|GetRespawnScreenREF)
    (:Is%20Valid
      (Widget|SetVisibility (Variables|Default|GetRespawnScreenREF) "Visible")
      (Default|StartTimer (Variables|Default|GetRespawnScreenREF)))
    (:Is%20Not%20Valid
      (bind _returnvalue (UserInterface|CreateWidget "/Game/UMG/Widgets/W_RespawnScreen.W_RespawnScreen_C" (Game|Player|GetOwningPlayerController)))
      (bind _output_get (Variables|Default|SetRespawnScreenREF _returnvalue))
      (UserInterface|Viewport|AddtoViewport _output_get 0))))

(event Custom|HideRespawnScreen
  (bind _respawnscreenref (Variables|Default|GetRespawnScreenREF))
  ;[0.2204 0 1] Show // Hide {W_RespawnScreen}
  (Widget|SetVisibility _respawnscreenref "Hidden")
  (Default|ResetTimer _respawnscreenref))

(event Custom|HitMarker
  ;[0 0.5344 1] Play HitMarker Animation from {W_HUD}
  (Default|HitMarkerAnimation (Variables|Default|GetHUDWidgetREF)))

(event Custom|SetMagazine
  (params (Magazine :type Integer))
  ;[0.9975 0.2871 1] Communicate Weapon Ammunition to {W_HUD}
  (Default|SetMagazine (Variables|Default|GetHUDWidgetREF) Magazine))

(event Custom|SetAmmo
  (params (Ammo :type Integer))
  ;[0.9975 0.2871 1] Communicate Weapon Ammunition to {W_HUD}
  (Default|SetAmmo (Variables|Default|GetHUDWidgetREF) Ammo))

(event Custom|ShowChatBox
  (params (TeamChat :type Boolean))
  (bind _hudwidgetref (Variables|Default|GetHUDWidgetREF))
  (bind _w_chatbox (Variables|/Game/UMG/Widgets/W_HUD.W_HUD_C|GetW_ChatBox _hudwidgetref))
  (bind _tab (Variables|/Game/UMG/Widgets/W_ChatBox.W_ChatBox_C|GetTab _w_chatbox))
  ;[0.2204 0 1] Show {W_ChatBox} - Global or Team - (automatically hides)
  (Widget|SetVisibility _w_chatbox "Visible")
  (Widget|SetVisibility (Variables|/Game/UMG/Widgets/W_ChatBox.W_ChatBox_C|GetChatEntry _w_chatbox) "Visible")
  (Class|Border|SetBrushColor (Variables|/Game/UMG/Widgets/W_ChatBox.W_ChatBox_C|GetChatContainer _w_chatbox) "(R=0.000000,G=0.000000,B=0.000000,A=0.250000)")
  (if TeamChat
    (Rendering|Components|TextRender|SetText _tab "TEAM")
    (Appearance|SetColorandOpacity _tab (Utilities|Struct|MakeSlateColor (Utilities|Select :Index (Variables|/Game/Blueprints/Characters/PC_FPS.PC_FPS_C|GetTeam (.AsPC%20FPS (Utilities|Casting|CastToPC_FPS (Game|GetPlayerController 0)))) :NewEnumerator0 "(R=1.000000,G=1.000000,B=1.000000,A=1.000000)" :NewEnumerator1 "(R=0.000000,G=0.226000,B=1.000000,A=1.000000)" :NewEnumerator2 "(R=1.000000,G=0.000000,B=0.000000,A=1.000000)")) :!class /Script/UMG.TextBlock)
    (else
      (Rendering|Components|TextRender|SetText _tab "GLOBAL")
      (Appearance|SetColorandOpacity _tab (Utilities|Struct|MakeSlateColor "(R=1.000000,G=1.000000,B=1.000000,A=1.000000)") :!class /Script/UMG.TextBlock))))

(event EventBeginPlay
  ;[0 0 1] BeginPlay
  (Utilities|FlowControl|Sequence
    (:then_0
      (bind _returnvalue (UserInterface|CreateWidget "/Game/UMG/Widgets/W_HUD.W_HUD_C"))
      (bind _output_get (Variables|Default|SetHUDWidgetREF _returnvalue))
      (UserInterface|Viewport|AddtoViewport _output_get 0))
    (:then_2
      (bind _returnvalue_2 (UserInterface|CreateWidget "/Game/UMG/Widgets/W_Timer.W_Timer_C"))
      (bind _output_get_2 (Variables|Default|SetTimer%20REF _returnvalue_2))
      (UserInterface|Viewport|AddtoViewport _output_get_2 0))))

(fn ConstructionScript)